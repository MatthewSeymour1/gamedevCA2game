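; Checkpoint actor that saves the player's data the first time the first-person character overlaps it.
; A saved flag makes it one-shot, so later overlaps only print a debug message.
; On that first overlap it plays a musical cue, activates the CheckpointPoof effect and shows a Checkpoint widget.
; It then calls SavePlayerData on the custom game instance, which handles the save itself.
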(event `self.ReceiveActorBeginOverlap`
  (params (OtherActor :type "Actor Object Reference"))
  (cast `/Game/FirstPerson/Blueprints/BP_FirstPersonCharacter` OtherActor)
  (if (`self.hasSavedAlready`)
    (`KismetSystemLibrary.PrintString` "don't save game")
    (else
      (set `self.hasSavedAlready` true)
      (`KismetSystemLibrary.PrintString` "save game")
      (`GameplayStatics.PlaySound2D` "/Game/Fab/Interface_And_Item_Sounds/Cues/Special_Musical_01_Cue.Special_Musical_01_Cue" 1.0 1.0 0.0 null null)
      (`ActorComponent.Activate` (`self.checkpointPoof`) false)
      (bind _returnvalue (`|CreateWidget` "/Game/Widgets/checkpoint.checkpoint_C" (`GameplayStatics.GetPlayerController` 0)))
      (`UserWidget.AddToViewport` _returnvalue 0)
      (bind _asmy_game_instance (cast `/Game/Blueprints/myGameInstance` (`GameplayStatics.GetGameInstance`)))
      (`/Game/Blueprints/myGameInstance.savePlayerData` _asmy_game_instance))))

(fn `UserConstructionScript`)