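; Time bomb projectile that the first-person player launches to place a TimeBombAOE where it lands.
; On BeginPlay it applies a velocity-change impulse to its sphere along the player camera's forward vector, scaled by TimeBombSpeed.
; On hit it destroys itself and all existing TimeBombAOE actors, then spawns a new one at the hit location, keeping one area active at a time.
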(event `self.ReceiveBeginPlay`
  (bind _asbp_first_person_character (cast `/Game/FirstPerson/Blueprints/BP_FirstPersonCharacter` (`GameplayStatics.GetPlayerCharacter` 0)))
  (`PrimitiveComponent.AddImpulse` (`self.Sphere`) (* (`SceneComponent.GetForwardVector` (`/Game/FirstPerson/Blueprints/BP_FirstPersonCharacter.FirstPersonCamera` _asbp_first_person_character)) (`self.timeBombSpeed`)) "None" true))

(event `self.Sphere.OnComponentHit`
  (params (HitComponent :type "PrimitiveComponent Object Reference") (OtherActor :type "Actor Object Reference") (OtherComp :type "PrimitiveComponent Object Reference") (NormalImpulse :type "Vector Structure") (Hit :type "HitResult Structure (by ref)"))
  (`self.K2_DestroyActor`)
  (bind _outactors (`GameplayStatics.GetAllActorsOfClass` "/Game/Blueprints/timeBombAOE.timeBombAOE_C"))
  (for _array_element _outactors
    (`self.K2_DestroyActor` _array_element))
  (`|SpawnActorFromClass` "/Game/Blueprints/timeBombAOE.timeBombAOE_C" (`KismetMathLibrary.Conv_VectorToTransform` Hit_Location) "Undefined" "MultiplyWithRoot" null null))

(fn `UserConstructionScript`)