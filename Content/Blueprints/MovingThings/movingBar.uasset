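; A spinning bar obstacle that knocks the first-person character away on contact.
; Tick advances the actor's yaw at the current speed, which the ApplySlow and RemoveSlow events switch between slowed and original values.
; On overlap it launches the character upward and away from its capsule, overriding velocity and printing the push direction, then ignores further hits for a short cooldown.
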(event `self.ReceiveActorBeginOverlap`
  (params (OtherActor :type "Actor Object Reference"))
  (bind _asbp_first_person_character (cast `/Game/FirstPerson/Blueprints/BP_FirstPersonCharacter` OtherActor))
  (if (`self.canHit`)
    (set `self.canHit` false)
    (bind _returnvalue (`KismetMathLibrary.Normal` (- (`SceneComponent.K2_GetComponentLocation` (`/Game/FirstPerson/Blueprints/BP_FirstPersonCharacter.FirstPersonMesh` _asbp_first_person_character)) (`SceneComponent.K2_GetComponentLocation` (`self.Capsule`)))))
    (`KismetSystemLibrary.PrintString` (`KismetStringLibrary.Conv_VectorToString` _returnvalue))
    (`Character.LaunchCharacter` _asbp_first_person_character (+ (* _returnvalue (`self.sidewaysPush`)) (0.0 0.0 1500.0)) true true)
    (`KismetSystemLibrary.Delay` 1.0)
    (set `self.canHit` true)))

(event `self.ReceiveBeginPlay`
  (set `self.currentSpeed` (`self.originalSpeed`)))

(event `self.ReceiveTick`
  (params (DeltaSeconds :type "Float (single-precision)"))
  (bind (_returnvalue_roll _returnvalue_pitch _returnvalue_yaw) (`KismetMathLibrary.BreakRotator` (`self.K2_GetActorRotation`)))
  (`self.K2_SetActorRotation` (`KismetMathLibrary.MakeRotator` _returnvalue_roll _returnvalue_pitch (+ _returnvalue_yaw (* DeltaSeconds (`self.currentSpeed`)))) true))

(event `/Game/Interfaces/slowFieldInterface.ApplySlow`
  (set `self.currentSpeed` (`self.slowSpeed`)))

(event `/Game/Interfaces/slowFieldInterface.RemoveSlow`
  (set `self.currentSpeed` (`self.originalSpeed`)))

(fn `UserConstructionScript`)