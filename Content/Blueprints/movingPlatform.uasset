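; Moving platform actor that travels back and forth along the world Y axis from its starting position.
; BeginPlay stores the start location, then Tick advances the Y position by Speed and Direction and moves the actor without sweep.
; Direction flips when the Y offset reaches MaxDistance or returns to zero, so motion stays on the positive side of the start.
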(event `self.ReceiveBeginPlay`
  (bind _output_get (set `self.startLocation` (`self.K2_GetActorLocation`)))
  (set `self.currentLocation` _output_get))

(event `self.ReceiveTick`
  (params (DeltaSeconds :type "Float (single-precision)"))
  (bind (_currentlocation_x _currentlocation_y) (`KismetMathLibrary.BreakVector` (`self.currentLocation`)))
  (bind (_startlocation_x _startlocation_y) (`KismetMathLibrary.BreakVector` (`self.startLocation`)))
  (bind (_currentlocation_x_2 _currentlocation_y_2 _currentlocation_z) (`KismetMathLibrary.BreakVector` (`self.currentLocation`)))
  (bind _output_get (set `self.currentLocation` (`KismetMathLibrary.MakeVector` _currentlocation_x_2 (+ _currentlocation_y_2 (* DeltaSeconds (`self.speed`) (`self.direction`))) _currentlocation_z)))
  (`self.K2_SetActorLocation` _output_get)
  (set `self.moveDistance` (- _currentlocation_y _startlocation_y))
  (if (> (`self.direction`) 0.0)
    (if (>= (`self.moveDistance`) (`self.maxDistance`))
      (set `self.direction` -1.0))
    (elif (<= (`self.moveDistance`) 0.0)
      (set `self.direction` 1.0))))

(fn `UserConstructionScript`)