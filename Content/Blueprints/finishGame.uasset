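; A trigger actor that ends the game when the first-person player character overlaps it.
; On overlap it removes the character's health and progress bar widgets and shows the EndMenu widget.
; It then switches input to UI only with the mouse cursor visible and pauses the game.
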(event `self.ReceiveActorBeginOverlap`
  (params (OtherActor :type "Actor Object Reference"))
  (bind _returnvalue (`GameplayStatics.GetPlayerController` 0))
  (bind _asbp_first_person_character (cast `/Game/FirstPerson/Blueprints/BP_FirstPersonCharacter` OtherActor))
  (`Widget.RemoveFromParent` (`/Game/FirstPerson/Blueprints/BP_FirstPersonCharacter.healthWidget Ref` _asbp_first_person_character))
  (`Widget.RemoveFromParent` (`/Game/FirstPerson/Blueprints/BP_FirstPersonCharacter.progressBarWidget Ref` _asbp_first_person_character))
  (bind _returnvalue_2 (`|CreateWidget` "/Game/Widgets/endMenu.endMenu_C" _returnvalue))
  (`UserWidget.AddToViewport` _returnvalue_2 0)
  (`WidgetBlueprintLibrary.SetInputMode_UIOnlyEx` _returnvalue _returnvalue_2)
  (set `PlayerController.bShowMouseCursor` true (`GameplayStatics.GetPlayerController` 0))
  (`GameplayStatics.SetGamePaused` true))

(fn `UserConstructionScript`)