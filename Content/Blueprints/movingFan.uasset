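; A fan actor that spins continuously and can be slowed down and restored.
; Tick adds the current speed, scaled by delta time, to the actor's roll while keeping pitch and yaw.
; BeginPlay starts it at the original speed, and the ApplySlow and RemoveSlow events switch the current speed between the slow and original values.
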(event `self.ReceiveBeginPlay`
  (set `self.currentSpeed` (`self.originalSpeed`)))

(event `self.ReceiveTick`
  (params (DeltaSeconds :type "Float (single-precision)"))
  (bind (_returnvalue_roll _returnvalue_pitch _returnvalue_yaw) (`KismetMathLibrary.BreakRotator` (`self.K2_GetActorRotation`)))
  (`self.K2_SetActorRotation` (`KismetMathLibrary.MakeRotator` (+ _returnvalue_roll (* DeltaSeconds (`self.currentSpeed`))) _returnvalue_pitch _returnvalue_yaw)))

(event `/Game/Interfaces/slowFieldInterface.ApplySlow`
  (set `self.currentSpeed` (`self.slowSpeed`)))

(event `/Game/Interfaces/slowFieldInterface.RemoveSlow`
  (set `self.currentSpeed` (`self.originalSpeed`)))

(fn `UserConstructionScript`)