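; Game instance that manages the first-person player's save game, persisting health and transform to a single slot.
; On Init it loads the existing save or creates a new save object, starting a looping autosave timer only when a save already existed.
; Functions write the character's state to the slot, restore it along with control rotation, or delete the slot.
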(event `self.ReceiveInit`
  (bind _slot_name (`self.Slot Name`))
  (bind _returnvalue (`GameplayStatics.DoesSaveGameExist` _slot_name))
  (if _returnvalue
    (bind _returnvalue_2 (`GameplayStatics.LoadGameFromSlot` _slot_name))
    (bind _assave_game_object (cast `/Game/Blueprints/saveGameObject` _returnvalue_2))
    (set `self.saveGameData` _assave_game_object)
    (`KismetSystemLibrary.K2_SetTimer` null "autoSave" 50.0 true)
    (else
      (bind _returnvalue_3 (`GameplayStatics.CreateSaveGameObject` "/Game/Blueprints/saveGameObject.saveGameObject_C"))
      (set `self.saveGameData` _returnvalue_3))))

(fn `autoSave`
  (`self.savePlayerData`))

(fn `clearData`
  (`GameplayStatics.DeleteGameInSlot` (`self.Slot Name`)))

(fn `loadPlayerData`
  (locals (PlayerRef :type "/Game/FirstPerson/Blueprints/BP_FirstPersonCharacter Object Reference"))
  (bind (_playersave_health _playersave_location) (break `/Game/Blueprints/playerSaveData` (`/Game/Blueprints/saveGameObject.playerSave` (`self.saveGameData`))))
  (bind _asbp_first_person_character (cast `/Game/FirstPerson/Blueprints/BP_FirstPersonCharacter` (`GameplayStatics.GetPlayerCharacter` 0)))
  (bind _output_get (set `local.PlayerRef` _asbp_first_person_character))
  (`Actor.K2_SetActorTransform` _output_get _playersave_location false false)
  (set `/Game/FirstPerson/Blueprints/BP_FirstPersonCharacter.health` _playersave_health _output_get)
  (`Controller.SetControlRotation` (`GameplayStatics.GetPlayerController` 0) (.rotation _playersave_location)))

(fn `savePlayerData`
  (locals (`Player Ref` :type "/Game/FirstPerson/Blueprints/BP_FirstPersonCharacter Object Reference"))
  (bind _asbp_first_person_character (cast `/Game/FirstPerson/Blueprints/BP_FirstPersonCharacter` (`GameplayStatics.GetPlayerCharacter` 0)))
  (bind _output_get (set `local.Player Ref` _asbp_first_person_character))
  (set `/Game/Blueprints/saveGameObject.playerSave` (make `/Game/Blueprints/playerSaveData` (`/Game/FirstPerson/Blueprints/BP_FirstPersonCharacter.health` _output_get) (`Actor.GetTransform` _output_get)) (`self.saveGameData`))
  (`GameplayStatics.SaveGameToSlot` (`self.saveGameData`) (`self.Slot Name`)))